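; Light control actor for the cartoon water shader pack that copies scene lighting into the MPC_LightData material parameter collection.
; UpdateLight writes the directional light's negated forward vector, intensity and color, plus the skylight's intensity and color, skipping invalid references.
; The construction script toggles tick via UpdateRealTime and runs UpdateLight only if the directional light is valid.
; Tick repeats the update for real-time lighting changes.
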(event `UpdateLight`
  (bind _directionalligth (`self.DirectionalLigth`))
  (bind _skylight (`self.SkyLight`))
  (bind _lightcomponent (`Light.LightComponent` _directionalligth))
  (bind _lightcomponent_2 (`SkyLight.LightComponent` _skylight))
  (bind (_returnvalue_x _returnvalue_y _returnvalue_z) (`KismetMathLibrary.BreakVector` (* (`KismetMathLibrary.GetForwardVector` (`SceneComponent.K2_GetComponentRotation` _lightcomponent)) -1.0)))
  (`|ExecutionSequence`
    (:`then_0`
      (`/Engine/EditorBlueprintResources/StandardMacros.IsValid` _directionalligth
        (:`Is Valid`
          (set `self.Directional Light Intensity` (`LightComponentBase.Intensity` _lightcomponent))
          (set `self.Directional Light Color` (`KismetMathLibrary.Conv_ColorToLinearColor` (`LightComponentBase.LightColor` _lightcomponent)))
          (`KismetMaterialLibrary.SetVectorParameterValue` "/ReturnToParadise/BoughtAssets/CartoonWaterShader/Materials/MaterialCollections/MPC_LightData.MPC_LightData" "Directional Light Vector" (make `LinearColor` _returnvalue_x _returnvalue_y _returnvalue_z 1.0))
          (`KismetMaterialLibrary.SetScalarParameterValue` "/ReturnToParadise/BoughtAssets/CartoonWaterShader/Materials/MaterialCollections/MPC_LightData.MPC_LightData" "Directional Ligth Intensity" (`self.Directional Light Intensity`))
          (`KismetMaterialLibrary.SetVectorParameterValue` "/ReturnToParadise/BoughtAssets/CartoonWaterShader/Materials/MaterialCollections/MPC_LightData.MPC_LightData" "Directional Light Color" (`self.Directional Light Color`)))))
    (:`then_1`
      (`/Engine/EditorBlueprintResources/StandardMacros.IsValid` _skylight
        (:`Is Valid`
          (set `self.SkyLight Intensity` (`LightComponentBase.Intensity` _lightcomponent_2))
          (set `self.SkyLight Color` (`KismetMathLibrary.Conv_ColorToLinearColor` (`LightComponentBase.LightColor` _lightcomponent_2)))
          (`KismetMaterialLibrary.SetScalarParameterValue` "/ReturnToParadise/BoughtAssets/CartoonWaterShader/Materials/MaterialCollections/MPC_LightData.MPC_LightData" "SkyLight Intensity" (`self.SkyLight Intensity`))
          (`KismetMaterialLibrary.SetVectorParameterValue` "/ReturnToParadise/BoughtAssets/CartoonWaterShader/Materials/MaterialCollections/MPC_LightData.MPC_LightData" "SkyLight Color" (`self.SkyLight Color`)))))))

(event `self.ReceiveTick`
  (params (DeltaSeconds :type "Float (single-precision)"))
  (`self.UpdateLight`))

(fn `UserConstructionScript`
  (`self.SetActorTickEnabled` (`self.UpdateRealTime`))
  (`/Engine/EditorBlueprintResources/StandardMacros.IsValid` (`self.DirectionalLigth`)
    (:`Is Valid`
      (`self.UpdateLight`))))