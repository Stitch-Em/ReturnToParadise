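; Cartoon sky actor that drives a day-night cycle for sun, moon, skylight and height fog.
; The selected cloud type picks the sky material in the construction script and the color curve set at BeginPlay.
; VEEvent time updates, rather than Tick, set sun pitch; sun elevation via dot product then samples those curves for light and fog colors.
; Optional editor preview uses StartHour; moon rotation and cheats are stubs, and networked time is unwired.
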(event `self.ReceiveBeginPlay`
  (bind _ve_event (`self.VE_Event`))
  (bind _ve_event_2 (`self.VE_Event`))
  (`|ExecutionSequence`
    (:`then_0`
      (add `/Game/VivaEngine/Core/EventManager/VE_EventManager.OnTimeUpdate` _ve_event_2 (delegate `TimeUpdate`))
      (add `/Game/VivaEngine/Core/EventManager/VE_EventManager.OnOneTimeEvent` _ve_event_2 (delegate `Cheats`))
      (bind _returnvalue (`GameplayStatics.GetActorOfClass` "/Script/Engine.SkyAtmosphere"))
      (`/Engine/EditorBlueprintResources/StandardMacros.IsValid` _returnvalue
        (:`Is Valid`
          _)
        (:`Is Not Valid`
          (`KismetSystemLibrary.PrintString` "Place Sky Atmosphere actor in the scene" true true (struct :`R` 1.0 :`A` 1.0) 30.0)))
      (switch `/ReturnToParadise/BoughtAssets/CartoonSkyShader/Blueprints/Data/E_CloudTypes` (`self.CloudTypes`)
        (:`NewEnumerator0`
          (set `self.Sun Light Color` (`self.Sun Light Color Type 1`) :!label _label)
          (set `self.Moon Light Color` (`self.Moon Light Color Type 1`))
          (set `self.Skylight Color` (`self.Skylight Color Type 1`))
          (set `self.Height Fog Color` (`self.Height Fog Type 1`)))
        (:`NewEnumerator1`
          (goto _label))
        (:`NewEnumerator2`
          (set `self.Sun Light Color` (`self.Sun Light Color Type 2`) :!label _label_2)
          (set `self.Moon Light Color` (`self.Moon Light Color Type 2`))
          (set `self.Skylight Color` (`self.Skylight Color Type 2`))
          (set `self.Height Fog Color` (`self.Height Fog Type 2`)))
        (:`NewEnumerator3`
          (goto _label_2))
        (:`NewEnumerator5`
          (set `self.Sun Light Color` (`self.Sun Light Color Type 3`) :!label _label_3)
          (set `self.Moon Light Color` (`self.Moon Light Color Type 3`))
          (set `self.Skylight Color` (`self.Skylight Color Type 3`))
          (set `self.Height Fog Color` (`self.Height Fog Type 3`)))
        (:`NewEnumerator6`
          (goto _label_3))
        (:`NewEnumerator7`
          (set `self.Sun Light Color` (`self.Sun Light Color Type 4`) :!label _label_4)
          (set `self.Moon Light Color` (`self.Moon Light Color Type 4`))
          (set `self.Skylight Color` (`self.Skylight Color Type 4`))
          (set `self.Height Fog Color` (`self.Height Fog Type 4`)))
        (:`NewEnumerator8`
          (goto _label_4))
        (:`NewEnumerator11`
          (set `self.Sun Light Color` (`self.Sun Light Color Type 5`) :!label _label_5)
          (set `self.Moon Light Color` (`self.Moon Light Color Type 5`))
          (set `self.Skylight Color` (`self.Skylight Color Type 5`))
          (set `self.Height Fog Color` (`self.Height Fog Type 5`)))
        (:`NewEnumerator12`
          (goto _label_5))))
    (:`then_1`
      (`/Game/VivaEngine/Core/EventManager/VE_EventManager.SetTime` _ve_event (`self.StartHour`) 0)
      (`self.Day Night Cycle` (`/Game/VivaEngine/Core/EventManager/VE_EventManager.Time` _ve_event)))))

(event `TimeUpdate`
  (params (Time :type "Timespan Structure"))
  (`self.Day Night Cycle` Time))

(event `Cheats`
  (params (Event :type "/Game/VivaEngine/Core/EventManager/VE_Event Structure"))
  (bind (_eventkey _eventvalue) (break `/Game/VivaEngine/Core/EventManager/VE_Event` Event))
  (bind ((`String_7_49BB567D4CB8BB14DC9E0EBE80B50DEE` _string) (`StarMenu_21_C47329EC4965B4F68A24718CD6B48685` _starmenu)) (break `/Game/VivaEngine/Core/EventManager/VE_Event_Storage` _eventvalue))
  (`self.RunCheats` (make `/Game/VivaEngine/Core/Hud/DebugMenu/VE_DebugActions` _eventkey _string _starmenu)))

(event `MulticastTime`)

(event `self.ReceiveTick`
  (params (DeltaSeconds :type "Float (single-precision)")))

(event `SetClientTime`
  (params (Time :type "Float (double-precision)"))
  (`self.Network Day Night Cycle` Time))

(fn `Day Night Cycle`
  (params (InTimespan :type "Timespan Structure"))
  (bind (_days _hours _minutes _seconds) (`KismetMathLibrary.BreakTimespan` InTimespan))
  (bind _moonlight (`self.MoonLight`))
  (bind _skylight (`self.Skylight`))
  (bind _height_fog (`self.Height Fog`))
  (bind _sunlight (`self.SunLight`))
  (bind _returnvalue (`KismetMathLibrary.NormalizeToRange` (+ (`KismetMathLibrary.Dot_VectorVector` (* (`SceneComponent.GetForwardVector` (`Light.LightComponent` _sunlight)) -1.0) (`SceneComponent.GetUpVector` (`self.Billboard`))) 0.5) 0.0 1.0))
  (`|ExecutionSequence`
    (:`then_0`
      (`/Engine/EditorBlueprintResources/StandardMacros.IsValid` _sunlight
        (:`Is Valid`
          (`SceneComponent.K2_SetWorldRotation` (`Actor.RootComponent` _sunlight) (`KismetMathLibrary.MakeRotator` 0.0 (`KismetMathLibrary.MapRangeClamped` (/ (+ (`KismetMathLibrary.Conv_IntToDouble` _hours) (`KismetMathLibrary.MapRangeClamped` (+ (`KismetMathLibrary.Conv_IntToDouble` _minutes) (`KismetMathLibrary.FClamp` (`KismetMathLibrary.MapRangeClamped` (`KismetMathLibrary.Conv_IntToDouble` _seconds) 0.0 60.0 0.0 1.0) 0.0 0.9999)) 0.0 60.0 0.0 0.9999)) 24.0) 0.0 1.0 0.0 360.0)) false true)
          (`LightComponent.SetLightColor` (`Light.LightComponent` _sunlight) (`CurveLinearColor.GetLinearColorValue` (`self.Sun Light Color`) _returnvalue) true)
          (`/Engine/EditorBlueprintResources/StandardMacros.IsValid` _skylight
            (:`Is Valid`
              (`SkyLightComponent.SetLightColor` (`SkyLight.LightComponent` _skylight) (`CurveLinearColor.GetLinearColorValue` (`self.Skylight Color`) _returnvalue))
              (`/Engine/EditorBlueprintResources/StandardMacros.IsValid` _height_fog
                (:`Is Valid`
                  (`ExponentialHeightFogComponent.SetFogInscatteringColor` (`ExponentialHeightFog.Component` _height_fog) (`CurveLinearColor.GetLinearColorValue` (`self.Height Fog Color`) _returnvalue)))
                (:`Is Not Valid`
                  (`KismetSystemLibrary.PrintString` "Set a Height Fog in BP_CartoonSky_DayNightCycle" false true (struct :`G` 0.66 :`B` 1.0 :`A` 1.0) 0.001))))
            (:`Is Not Valid`
              (`KismetSystemLibrary.PrintString` "Set a Sky Light in BP_CartoonSky_DayNightCycle" false true (struct :`G` 0.66 :`B` 1.0 :`A` 1.0) 0.001))))
        (:`Is Not Valid`
          (`KismetSystemLibrary.PrintString` "Set a Sun Light in BP_CartoonSky_DayNightCycle" false true (struct :`G` 0.66 :`B` 1.0 :`A` 1.0) 0.001))))
    (:`then_1`
      (`/Engine/EditorBlueprintResources/StandardMacros.IsValid` _moonlight
        (:`Is Valid`
          (`LightComponent.SetLightColor` (`Light.LightComponent` _moonlight) (`CurveLinearColor.GetLinearColorValue` (`self.Moon Light Color`) _returnvalue) true)
          (if (`self.Moon Rotation?`)
            _))
        (:`Is Not Valid`
          (`KismetSystemLibrary.PrintString` "Set a Moon Light in BP_CartoonSky_DayNightCycle" false true (struct :`G` 0.66 :`B` 1.0 :`A` 1.0) 0.001))))))

(fn `Network Day Night Cycle`
  (params (Time :type "Float (double-precision)"))
  (`self.K2_SetActorRotation` (`self.SunLight`) (`KismetMathLibrary.MakeRotator` 0.0 (`KismetMathLibrary.FWrap` (`KismetMathLibrary.MapRangeUnclamped` Time 0.0 1.0 0.0 360.0) 0.0 360.0)) true))

(fn `RunCheats`
  (params (Action :type "/Game/VivaEngine/Core/Hud/DebugMenu/VE_DebugActions Structure")))

(fn `UserConstructionScript`
  (bind _ve_event (`self.VE_Event`))
  (`PrimitiveComponent.SetMaterial` (`self.CartoonSky`) 0 (select `/ReturnToParadise/BoughtAssets/CartoonSkyShader/Blueprints/Data/E_CloudTypes` (`self.CloudTypes`) :`NewEnumerator0` "/ReturnToParadise/BoughtAssets/CartoonSkyShader/Materials/CartoonSkyInstances/MI_CartoonSky_Type_1_High_Detail.MI_CartoonSky_Type_1_High_Detail" :`NewEnumerator1` "/ReturnToParadise/BoughtAssets/CartoonSkyShader/Materials/CartoonSkyInstances/MI_CartoonSky_Type_Viva_Low_Detail.MI_CartoonSky_Type_Viva_Low_Detail" :`NewEnumerator2` "/ReturnToParadise/BoughtAssets/CartoonSkyShader/Materials/CartoonSkyInstances/MI_CartoonSky_Type_2_High_Detail.MI_CartoonSky_Type_2_High_Detail" :`NewEnumerator3` "/ReturnToParadise/BoughtAssets/CartoonSkyShader/Materials/CartoonSkyInstances/MI_CartoonSky_Type_2_Low_Detail.MI_CartoonSky_Type_2_Low_Detail" :`NewEnumerator5` "/ReturnToParadise/BoughtAssets/CartoonSkyShader/Materials/CartoonSkyInstances/MI_CartoonSky_Type_3_High_Detail.MI_CartoonSky_Type_3_High_Detail" :`NewEnumerator6` "/ReturnToParadise/BoughtAssets/CartoonSkyShader/Materials/CartoonSkyInstances/MI_CartoonSky_Type_3_Low_Detail.MI_CartoonSky_Type_3_Low_Detail" :`NewEnumerator7` "/ReturnToParadise/BoughtAssets/CartoonSkyShader/Materials/CartoonSkyInstances/MI_CartoonSky_Type_4_High_Detail.MI_CartoonSky_Type_4_High_Detail" :`NewEnumerator8` "/ReturnToParadise/BoughtAssets/CartoonSkyShader/Materials/CartoonSkyInstances/MI_CartoonSky_Type_4_Low_Detail.MI_CartoonSky_Type_4_Low_Detail" :`NewEnumerator11` "/ReturnToParadise/BoughtAssets/CartoonSkyShader/Materials/CartoonSkyInstances/MI_CartoonSky_Type_5_High_Detail.MI_CartoonSky_Type_5_High_Detail" :`NewEnumerator12` "/ReturnToParadise/BoughtAssets/CartoonSkyShader/Materials/CartoonSkyInstances/MI_CartoonSky_Type_5_Low_Detail.MI_CartoonSky_Type_5_Low_Detail" :!type "MaterialInterface Object Reference"))
  (if (`self.Update Sky in the editor`)
    (`/Game/VivaEngine/Core/EventManager/VE_EventManager.SetTime` _ve_event (`self.StartHour`) 0)
    (`self.Day Night Cycle` (`/Game/VivaEngine/Core/EventManager/VE_EventManager.Time` _ve_event))))