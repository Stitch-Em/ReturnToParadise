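; Actor component that steers a flying AI actor around obstacles toward a target set by Server_MoveTo, without a navmesh.
; A looping timer capsule-traces to the target and, if blocked, sweeps a horizontal ring plus an optional randomly up/down-pitched ring, picking the candidate nearest the target.
; Optional explored-location memory rejects hit points near previously visited spots.
; Tick interpolates rotation and swept movement toward that waypoint until arrival stops the timer.
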(event `self.ReceiveBeginPlay`
  ;[1 1 1] At Component Beginning, store the owner actor for use
  (set `self.OwnerAIActor` (`self.GetOwner`)))

(event `Server_MoveTo`
  (params (Location :type "Vector Structure"))
  ;[1 1 1] Update Move To Location
  (set `self.TargetLocation` Location)
  ;[1 1 1] Start a timer for updating movement
  (bind _returnvalue (`KismetSystemLibrary.K2_SetTimerDelegate` (delegate `MovementUpdaterTimer`) (`self.PathTraceInterval`) true))
  (set `self.MovementTimerHandler` _returnvalue))

(event `MovementUpdaterTimer`
  ;[1 1 1] Start a timer for updating movement
  (`self.Server_UpdateMovement`))

(event `Server_UpdateMovement`
  ;[1 1 1] Code to update movement and rotation of the AI Actor
  ;;[1 1 1] Check if the location reached acceptance was reached
  (if (<= (`KismetMathLibrary.Abs` (`KismetMathLibrary.VSize` (- (`Actor.K2_GetActorLocation` (`self.OwnerAIActor`)) (`self.TargetLocation`)))) (`self.LocationReachedAcceptance`))
    ;;[1 1 1] Once path goal is reached, stop pathfinding algorithm and clear the explored areas
    (`KismetSystemLibrary.K2_ClearAndInvalidateTimerHandle` (`self.MovementTimerHandler`))
    (`KismetArrayLibrary.Array_Clear` (`self.ExploredAreas`))
    (else
      ;;[1 1 1] Find Closest Point To Target Location Without Geometry Blocking the Way
      (bind _location (`self.FindClosestDirectPointToTarget` (`self.TargetLocation`)))
      (set `self.CurrentMoveLocation` _location)
      (`self.AddExploredArea`))))

(event `self.ReceiveTick`
  (params (DeltaSeconds :type "Float (single-precision)"))
  (bind _returnvalue (`GameplayStatics.GetWorldDeltaSeconds`))
  (bind _owneraiactor (`self.OwnerAIActor`))
  ;[1 1 1] Code to update movement and rotation of the AI Actor
  ;;[1 1 1] Update Rotation To Movement Direction
  (if (`KismetSystemLibrary.K2_IsTimerActiveHandle` (`self.MovementTimerHandler`))
    (`Actor.K2_SetActorRotation` (`self.OwnerAIActor`) (`KismetMathLibrary.RInterpTo` (`Actor.K2_GetActorRotation` _owneraiactor) (`KismetMathLibrary.FindLookAtRotation` (`Actor.K2_GetActorLocation` _owneraiactor) (`self.CurrentMoveLocation`)) _returnvalue (`self.RotationSpeed`)) false)
    ;;[1 1 1] Move To Current Move Location
    (`Actor.K2_SetActorLocation` (`self.OwnerAIActor`) (`KismetMathLibrary.VInterpTo_Constant` (`Actor.K2_GetActorLocation` (`self.OwnerAIActor`)) (`self.CurrentMoveLocation`) _returnvalue (`self.ActorMovementSpeed`)) true false)))

(fn `AddExploredArea`
  (bind _exploredareas (`self.ExploredAreas`))
  (if (> (`KismetArrayLibrary.Array_Length` _exploredareas) (`self.MaxExploredLocationsStored`))
    (`KismetArrayLibrary.Array_Remove` (`self.ExploredAreas`)))
  (`KismetArrayLibrary.Array_Add` _exploredareas (`Actor.K2_GetActorLocation` (`self.OwnerAIActor`))))

(fn `FindClosestDirectPointToTarget`
  (params (TargetLocation :type "Vector Structure"))
  (returns (Location :type "Vector Structure"))
  (locals (ObstaclesDetectedHits :type "Array of Vector Structure") (FindRadious :type "Float (double-precision)") (ClosestDistance :type "Float (double-precision)" :default 999999995904.0) (ClosestMoveLocation :type "Vector Structure"))
  (bind _traceradious (`self.TraceRadious`))
  (bind _traceradious_2 (`self.TraceRadious`))
  (bind _traceradious_3 (`self.TraceRadious`))
  (bind _verticleangletracing (`self.VerticleAngleTracing`))
  (set `local.FindRadious` (`KismetMathLibrary.Abs` (`KismetMathLibrary.VSize` (- (`Actor.K2_GetActorLocation` (`self.OwnerAIActor`)) TargetLocation)))) ; Decides how far does the AI need to trace to find obstacles in its path
  (bind _outhit (`KismetSystemLibrary.CapsuleTraceSingle` :`Start` (`Actor.K2_GetActorLocation` (`self.OwnerAIActor`)) :`End` (`local.TargetLocation`) :`Radius` _traceradious_3 :`HalfHeight` _traceradious_3 :`TraceChannel` (`self.FinderCollisionChannel`) :`bTraceComplex` true :`DrawDebugType` (select `bool` (`self.EnableTraceDebugging?`) :`true` "ForDuration" :!type "EDrawDebugTrace Enum") :`DrawTime` (`self.PathTraceInterval`)))
  (if (`GameplayStatics.BreakHitResult` _outhit)
    (for _index (range 36)
      (bind _outhit_2 (`KismetSystemLibrary.CapsuleTraceSingle` :`Start` (`Actor.K2_GetActorLocation` (`self.OwnerAIActor`)) :`End` (+ (* (`KismetMathLibrary.GreaterGreater_VectorRotator` (1.0 0.0 0.0) (`KismetMathLibrary.MakeRotator` 0.0 0.0 (* _index 10.0))) (`local.FindRadious`)) (`Actor.K2_GetActorLocation` (`self.GetOwner`))) :`Radius` _traceradious :`HalfHeight` _traceradious :`TraceChannel` (`self.FinderCollisionChannel`) :`bTraceComplex` true :`DrawDebugType` (select `bool` (`self.EnableTraceDebugging?`) :`true` "ForDuration" :!type "EDrawDebugTrace Enum") :`DrawTime` (`self.PathTraceInterval`)))
      (bind (_bblockinghit _binitialoverlap _time _distance _location _impactpoint _normal _impactnormal _physmat _hitactor _hitcomponent _hitbonename _bonename _hititem _elementindex _faceindex _tracestart _traceend) (`GameplayStatics.BreakHitResult` _outhit_2))
      (if _bblockinghit
        (bind _returnvalue (+ _impactpoint (* _impactnormal 50.0)))
        (bind _alreadyexplored_ (`self.IsLocationAlreadyExplored?` _returnvalue))
        (if (not _alreadyexplored_)
          (`KismetArrayLibrary.Array_Add` (`local.ObstaclesDetectedHits`) _returnvalue))
        (else
          (`KismetArrayLibrary.Array_Add` (`local.ObstaclesDetectedHits`) _traceend))))
    (if (`self.TraceVerticalObstacles?`)
      (for _index_2 (range 36)
        (bind _outhit_3 (`KismetSystemLibrary.CapsuleTraceSingle` :`Start` (`Actor.K2_GetActorLocation` (`self.OwnerAIActor`)) :`End` (+ (* (`KismetMathLibrary.GreaterGreater_VectorRotator` (1.0 0.0 0.0) (`KismetMathLibrary.MakeRotator` 0.0 (select `bool` (`KismetMathLibrary.RandomBool`) :`false` (* _verticleangletracing -1.0) :`true` _verticleangletracing) (* _index_2 10.0))) (* (`local.FindRadious`) (`self.VerticalTraceRangeMultiplier`))) (`Actor.K2_GetActorLocation` (`self.GetOwner`))) :`Radius` _traceradious_2 :`HalfHeight` _traceradious_2 :`TraceChannel` (`self.FinderCollisionChannel`) :`bTraceComplex` true :`DrawDebugType` (select `bool` (`self.EnableTraceDebugging?`) :`true` "ForDuration" :!type "EDrawDebugTrace Enum") :`DrawTime` (`self.PathTraceInterval`)))
        (bind (_bblockinghit_2 _binitialoverlap_2 _time_2 _distance_2 _location_2 _impactpoint_2 _normal_2 _impactnormal_2 _physmat_2 _hitactor_2 _hitcomponent_2 _hitbonename_2 _bonename_2 _hititem_2 _elementindex_2 _faceindex_2 _tracestart_2 _traceend_2) (`GameplayStatics.BreakHitResult` _outhit_3))
        (if _bblockinghit_2
          (bind _returnvalue_2 (+ _impactpoint_2 (* _impactnormal_2 50.0)))
          (bind _alreadyexplored__2 (`self.IsLocationAlreadyExplored?` _returnvalue_2))
          (if (not _alreadyexplored__2)
            (`KismetArrayLibrary.Array_Add` (`local.ObstaclesDetectedHits`) _returnvalue_2))
          (else
            (`KismetArrayLibrary.Array_Add` (`local.ObstaclesDetectedHits`) _traceend_2)))))
    (for _array_element (`local.ObstaclesDetectedHits`)
      (bind _returnvalue_3 (`KismetMathLibrary.Abs` (`KismetMathLibrary.VSize` (- _array_element (`local.TargetLocation`)))))
      (if (< _returnvalue_3 (`local.ClosestDistance`))
        (set `local.ClosestDistance` _returnvalue_3)
        (set `local.ClosestMoveLocation` _array_element)))
    (return (`local.ClosestMoveLocation`))
    (else
      (return (`local.TargetLocation`)))))

(fn `IsLocationAlreadyExplored?`
  (params (Location :type "Vector Structure"))
  (returns (`AlreadyExplored?` :type Boolean))
  (if (`self.EnableComplexPathfinding?`)
    (for _array_element (`self.ExploredAreas`)
      (if (== _array_element (`local.Location`) :`ErrorTolerance` (`self.LocationExploredThreshold`))
        (return true)))
    (return false)
    (else
      (return false))))