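; Test Blueprint that drives a fur-physics material on a skeletal mesh from a moving sphere.
; BeginPlay spawns a VE_FurPhysicsTest sphere actor and snaps it to socket P1.
; Tick feeds its radius and location into a dynamic PhysicsTest material created in the construction script.
; It also derives a trailing direction and remapped per-frame travel distance from the previous position for the material, printing that distance for debugging.
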(event `self.ReceiveBeginPlay`
  (bind _returnvalue (`|SpawnActorFromClass` "/Game/VivaEngine/Core/Graphics/Fur/VE_FurPhysicsTest.VE_FurPhysicsTest_C" (`KismetMathLibrary.MakeTransform` (0.0 0.0 10000.0)) "AlwaysSpawn" "MultiplyWithRoot" null null))
  (`SphereComponent.SetSphereRadius` (`/Game/VivaEngine/Core/Graphics/Fur/VE_FurPhysicsTest.Sphere` _returnvalue) 200.0 true)
  (`self.K2_AttachToComponent` _returnvalue (`self.SkeletalMesh`) "P1" "SnapToTarget" "SnapToTarget" "SnapToTarget" true))

(event `self.ReceiveTick`
  (params (DeltaSeconds :type "Float (single-precision)"))
  (bind _cp (`self.CP`))
  (bind _pp (`self.PP`))
  (bind _material (`self.Material`))
  (bind _returnvalue (`KismetMathLibrary.Vector_Distance` _pp _cp))
  (bind _returnvalue_2 (`GameplayStatics.GetActorOfClass` "/Game/VivaEngine/Core/Graphics/Fur/VE_FurPhysicsTest.VE_FurPhysicsTest_C"))
  (`MaterialInstanceDynamic.SetScalarParameterValue` _material "Radius1" (`SphereComponent.GetUnscaledSphereRadius` (`/Game/VivaEngine/Core/Graphics/Fur/VE_FurPhysicsTest.Sphere` _returnvalue_2)))
  (bind _sphere (`/Game/VivaEngine/Core/Graphics/Fur/VE_FurPhysicsTest.Sphere` _returnvalue_2))
  (`MaterialInstanceDynamic.SetVectorParameterValue` _material "Location1" (`KismetMathLibrary.Conv_VectorToLinearColor` (`SceneComponent.K2_GetComponentLocation` _sphere)))
  (bind _returnvalue_3 (`SceneComponent.K2_GetComponentLocation` _sphere))
  (set `self.CP` _returnvalue_3)
  (`MaterialInstanceDynamic.SetVectorParameterValue` _material "V1" (`KismetMathLibrary.Conv_VectorToLinearColor` (`KismetMathLibrary.GetDirectionUnitVector` _cp _pp)))
  (`MaterialInstanceDynamic.SetScalarParameterValue` _material "VA" (`KismetMathLibrary.MapRangeUnclamped` _returnvalue 0.0 3.0 0.0 10.0))
  (`KismetSystemLibrary.PrintString` (`KismetStringLibrary.Conv_DoubleToString` _returnvalue) true true (struct :`G` 0.66 :`B` 1.0 :`A` 1.0) 2.0 "a")
  (set `self.PP` _returnvalue_3))

(fn `UserConstructionScript`
  (bind _returnvalue (`PrimitiveComponent.CreateDynamicMaterialInstance` (`self.SkeletalMesh`) 0 "/Game/VivaEngine/Core/Graphics/Fur/PhysicsTest.PhysicsTest" "None"))
  (set `self.Material` _returnvalue)
  (bind _returnvalue_2 (`GameplayStatics.GetActorOfClass` "/Game/VivaEngine/Core/Graphics/Fur/VE_FurPhysicsTest.VE_FurPhysicsTest_C"))
  (`MaterialInstanceDynamic.SetScalarParameterValue` _returnvalue "Radius1" (`SphereComponent.GetUnscaledSphereRadius` (`/Game/VivaEngine/Core/Graphics/Fur/VE_FurPhysicsTest.Sphere` _returnvalue_2)))
  (`MaterialInstanceDynamic.SetVectorParameterValue` _returnvalue "Location1" (`KismetMathLibrary.Conv_VectorToLinearColor` (`SceneComponent.K2_GetComponentLocation` (`/Game/VivaEngine/Core/Graphics/Fur/VE_FurPhysicsTest.Sphere` _returnvalue_2)))))